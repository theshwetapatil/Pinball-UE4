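; Pinball drop target actor that sinks when hit, labeled with a configurable letter set in the construction script.
; Hit calls Drop, which moves the mesh down, disables its collision and plays a bumper sound, then fires the OnDrop dispatcher.
; Reset_Target raises the mesh and restores collision.
; BeginPlay binds an event to the pinball game mode's OnGameReset dispatcher.
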(event Custom|Drop
  (Components|MoveComponentTo (Variables|Default|GetDT_Mesh) "0, 0,-110.000000" "0, 0, 0" false false 0.2 false)
  (Collision|SetCollisionEnabled (Variables|Default|GetDT_Mesh) "NoCollision")
  (Audio|PlaySoundatLocation "/Game/Assets/Sounds/Bumper_Hit.Bumper_Hit" (Transformation|GetActorLocation)))

(event Custom|Reset_Target
  (Components|MoveComponentTo (Variables|Default|GetDT_Mesh) "0, 0,0.000000" "0, 0, 0" false false 0.2 false)
  (Collision|SetCollisionEnabled (Variables|Default|GetDT_Mesh) "QueryAndPhysics"))

(event Collision|EventActorBeginOverlap
  (params (OtherActor :type Actor%20Object%20Reference)))

(event EventTick
  (params (DeltaSeconds :type Float%20%28single-precision%29)))

(event EventBeginPlay
  (bind _aspinball_game_mode_blueprint (Utilities|Casting|CastToPinball_Game_Mode_Blueprint (Game|GetGameMode)))
  (EventDispatchers|BindEventtoOnGameReset _aspinball_game_mode_blueprint (EventDispatchers|CreateEvent :!event Custom|Reset_Target)))

(event Collision|EventHit
  (params (MyComp :type Primitive%20Component%20Object%20Reference) (Other :type Actor%20Object%20Reference) (OtherComp :type Primitive%20Component%20Object%20Reference) (bSelfMoved :type Boolean) (HitLocation :type Vector :default "0, 0, 0") (HitNormal :type Vector :default "0, 0, 0") (NormalImpulse :type Vector :default "0, 0, 0") (Hit :type Hit%20Result%20Structure%20%28by%20ref%29))
  (CallFunction|Drop)
  (Default|CallOnDrop))

(fn ConstructionScript
  (Rendering|Components|TextRender|SetText (Variables|Default|GetTextRender) (Utilities|Text|ToText(String) (Variables|Default|GetDrop_Letter))))