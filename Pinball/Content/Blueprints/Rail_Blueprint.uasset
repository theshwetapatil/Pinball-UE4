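; Rail Blueprint that builds a rail along an editable spline, entirely in the Construction Script with no runtime logic.
; It adds one spline mesh component per segment, aligned to the local location and tangent of both spline points.
; The first segment uses the start mesh with an adjustable X start scale, the last uses the end mesh, and those between use the middle mesh.
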(event EventBeginPlay)

(event Collision|EventActorBeginOverlap
  (params (OtherActor :type Actor%20Object%20Reference)))

(event EventTick
  (params (DeltaSeconds :type Float%20%28single-precision%29)))

(fn ConstructionScript
  (bind _spline (Variables|Default|GetSpline))
  (bind _spline_2 (Variables|Default|GetSpline))
  (bind _returnvalue (Spline|GetNumberOfSplinePoints _spline))
  (bind _returnvalue_2 (- _returnvalue 2))
  (for _index (range 0 _returnvalue_2)
    (bind _returnvalue_3 (AddComponent|AddSplineMeshComponent false))
    (if (== _index 0)
      (Components|StaticMesh|SetStaticMesh _returnvalue_3 (Variables|Default|GetRail_Start_Mesh))
      (SplineMesh|SetStartScale _returnvalue_3 (Math|Vector2D|MakeVector2D (Variables|Default|GetInitial_Scale) 1.0) true :!class /Script/Engine.SplineMeshComponent)
      (elif (== _index _returnvalue_2)
        (Components|StaticMesh|SetStaticMesh _returnvalue_3 (Variables|Default|GetRail_End_Mesh))
        (else
          (Components|StaticMesh|SetStaticMesh _returnvalue_3 (Variables|Default|GetRail_Mid_Mesh)))))
    (SplineMesh|SetStartandEnd _returnvalue_3 (.Location (Spline|GetLocationandTangentatSplinePoint _spline_2 _index "Local")) (.Tangent (Spline|GetLocationandTangentatSplinePoint _spline_2 _index "Local")) (.Location (Spline|GetLocationandTangentatSplinePoint _spline_2 (+ _index 1) "Local")) (.Tangent (Spline|GetLocationandTangentatSplinePoint _spline_2 (+ _index 1) "Local")) true :!class /Script/Engine.SplineMeshComponent)))