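; Pinball ball Blueprint that rolls across the table under constant pull and plays motion-driven audio.
; Each Tick applies a DefaultSpeed velocity impulse, then traces downward and pushes the ball against the hit surface normal, scaled by TableStickiness, to keep it on the table.
; Tick also maps the ball's velocity to the rolling sound's clamped volume and pitch.
; BeginPlay plays a ball-loose cue attached to the ball.
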(event EventBeginPlay
  (Audio|SpawnSoundAttached "/Game/Assets/Sounds/Pinball_BallLoose_Cue.Pinball_BallLoose_Cue" (Variables|Default|GetBall)))

(event Collision|EventActorBeginOverlap
  (params (OtherActor :type Actor%20Object%20Reference)))

(event EventTick
  (params (DeltaSeconds :type Float%20%28single-precision%29))
  (bind _returnvalue (Transformation|GetActorLocation))
  (bind _returnvalue_2 (Transformation|GetVelocity))
  (bind _ball_rolling_sound (Variables|Default|GetBall_Rolling_Sound))
  (bind _returnvalue_3 (Math|Vector|VectorLength _returnvalue_2))
  (bind _returnvalue_4 (/ _returnvalue_3 1e+03))
  (Utilities|FlowControl|Sequence
    (:then_0
      (Physics|AddImpulse (Variables|Default|GetBall) (* (Variables|Default|GetDefaultSpeed) DeltaSeconds) "None" true)
      (bind _outhit (Collision|LineTraceByChannel _returnvalue (- _returnvalue "0, 0,500.000000") "TraceTypeQuery1" false 0 "None"))
      (Physics|AddImpulse (Variables|Default|GetBall) (* (* (.ImpactNormal (Collision|BreakHitResult _outhit)) -1) (* (Variables|Default|GetTableStickiness) DeltaSeconds)) "None" true))
    (:then_1
      (Audio|Components|Audio|SetVolumeMultiplier _ball_rolling_sound (Math|Float|Clamp(Float) _returnvalue_4) :!class /Script/Engine.AudioComponent)
      (Audio|Components|Audio|SetPitchMultiplier _ball_rolling_sound (Math|Float|Clamp(Float) _returnvalue_4 0.97 1.2)))))

(fn ConstructionScript)