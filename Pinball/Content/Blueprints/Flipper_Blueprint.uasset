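; Pinball-style flipper actor whose Flipper component rotates between a resting and a flipped angle.
; The construction script picks start and end rotations from a Left or Right FlipType, sets the resting pose, and mirrors right flippers with negative X scale.
; Flip and Flop events use MoveComponentTo to rotate to the end or start rotation over FlipTime.
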(event Custom|Flip
  (Components|MoveComponentTo (Variables|Default|GetFlipper) "0, 0, 0" (Variables|Default|GetEnd_Rotation) false false (Variables|Default|GetFlip_Time) false) ; Within the given period moves the component\nfrom it's location to the target location
)

(event Custom|Flop
  (Components|MoveComponentTo (Variables|Default|GetFlipper) "0, 0, 0" (Variables|Default|GetStart_Rotation) false false (Variables|Default|GetFlip_Time) false) ; Within the given period moves the component\nfrom it's location to the target location
)

(event EventBeginPlay)

(event Collision|EventActorBeginOverlap
  (params (OtherActor :type Actor%20Object%20Reference)))

(event EventTick
  (params (DeltaSeconds :type Float%20%28single-precision%29)))

(fn ConstructionScript
  (Variables|Default|SetStart_Rotation (Utilities|Select :Index (Variables|Default|GetFlip_Type) :NewEnumerator0 "0,20.000000, 0" :NewEnumerator1 "0,-20.000000, 0"))
  (Variables|Default|SetEnd_Rotation (Utilities|Select :Index (Variables|Default|GetFlip_Type) :NewEnumerator0 "0,-20.000000, 0" :NewEnumerator1 "0,20.000000, 0"))
  (Transformation|SetRelativeRotation (Variables|Default|GetFlipper) (Variables|Default|GetStart_Rotation) false false)
  (switch Utilities|FlowControl|Switch|SwitchonFlip_Type (Variables|Default|GetFlip_Type) ; If it's Right, Flip it
    (:NewEnumerator1
      (Transformation|SetRelativeScale3D (Variables|Default|GetFlipper) "-1.000000,1.000000,1.000000") ; To mirror Flipper from the pivot point
    )))