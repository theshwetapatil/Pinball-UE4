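; Pinball game mode that runs the match loop: main menu and music at start, score with multiplier, ball count and game reset.
; Spawns balls at the first plunger and binds each one's destroy event to respawn it or end the game when none remain.
; At game end, lazily loaded or created save data decides between the high score entry widget and a return to the main menu.
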(event Custom|Spawn_Ball
  (bind _outactors (Actor|GetAllActorsOfClass "/Game/Blueprints/Plunger_Blueprint.Plunger_Blueprint_C"))
  (bind _returnvalue (Game|SpawnActorfromClass "/Game/Blueprints/Ball_Blueprint.Ball_Blueprint_C" (Math|Transform|MakeTransform (Default|GetBallSpawnLocation (Utilities|Array|Get(acopy) _outactors)) "0, 0, 0" "1,1,1") "Undefined" 0 0))
  (Game|BindEventtoOnDestroyed _returnvalue (delegate Custom|On_Ball_Destroyed)) ; Caused by an event dispatcher\nAllows to get a message, \nfrom the ball\nwhen it gets destroyed
)

(event Custom|Create_High_Score_List
  (bind _returnvalue (Game|GetPlayerController 0))
  (bind _aspinball_player_controller_blueprint (Utilities|Casting|CastToPinball_Player_Controller_Blueprint _returnvalue))
  (bind _returnvalue_2 (UserInterface|CreateWidget "/Game/Blueprints/High_Score_Entry_WidgetBlueprint.High_Score_Entry_WidgetBlueprint_C" _aspinball_player_controller_blueprint))
  (UserInterface|Viewport|AddtoViewport _returnvalue_2 0)
  (Variables|/Script/Engine.PlayerController|SetbShowMouseCursor _aspinball_player_controller_blueprint true))

(event Custom|Create_Main_Menu
  (bind _returnvalue (Game|GetPlayerController 0))
  (bind _aspinball_player_controller_blueprint (Utilities|Casting|CastToPinball_Player_Controller_Blueprint _returnvalue))
  (CallFunction|GetSaveGameData)
  (Viewport|RemoveAllWidgets)
  (bind _returnvalue_2 (UserInterface|CreateWidget "/Game/Blueprints/Main_Menu_WidgetBlueprint.Main_Menu_WidgetBlueprint_C" _aspinball_player_controller_blueprint))
  (UserInterface|Viewport|AddtoViewport _returnvalue_2 0)
  (Variables|/Script/Engine.PlayerController|SetbShowMouseCursor _aspinball_player_controller_blueprint true))

(event Custom|On_Ball_Destroyed
  (params (DestroyedActor :type Actor%20Object%20Reference))
  (if (> (Variables|Default|GetBalls_Remaining) 0)
    (CallFunction|SpawnBall)
    (Math|Integer|DecrementInt (Variables|Default|GetBalls_Remaining))
    (else
      (CallFunction|EndGame))))

(event Custom|Reset_Game
  (bind _returnvalue (Game|GetPlayerController 0))
  (bind (_score _multiplier _balls_remaining) (Utilities|GetClassDefaults "Pinball_Game_Mode_Blueprint_C"))
  (bind _aspinball_player_controller_blueprint (Utilities|Casting|CastToPinball_Player_Controller_Blueprint _returnvalue))
  (Variables|Default|SetScore _score)
  (Variables|Default|SetMultiplier _multiplier)
  (Variables|Default|SetBalls_Remaining _balls_remaining)
  (CallFunction|SpawnBall)
  (Default|CreatePlayerHUD _aspinball_player_controller_blueprint)
  (Variables|/Script/Engine.PlayerController|SetbShowMouseCursor _aspinball_player_controller_blueprint false)
  (Default|CallOnGameReset))

(event Custom|End_Game
  (bind _current_save_object (CallFunction|GetSaveGameData))
  (if (<= (Utilities|Array|Length (Variables|/Game/Blueprints/High_Score_Save_Blueprint.High_Score_Save_Blueprint_C|GetSave_Struct _current_save_object)) 3)
    (CallFunction|CreateHighScoreList :!label _label)
    (else
      (bind _lowest_score_struct (Default|DetermineLowestScoreValue _current_save_object))
      (if (< (.score _lowest_score_struct) (Variables|Default|GetScore))
        (goto _label)
        (else
          (CallFunction|CreateMainMenu))))))

(event EventBeginPlay
  (CallFunction|CreateMainMenu)
  (Audio|PlaySound2D "/Game/Assets/Sounds/victoryMusic_loop_01_01.victoryMusic_loop_01_01" 0.2))

(event EventTick
  (params (DeltaSeconds :type Float%20%28single-precision%29)))

(fn ConstructionScript)

(fn AddScore
  (params (Points_To_Add :type Float%20%28single-precision%29))
  (bind _output_get (Variables|Default|SetScore (+ (* Points_To_Add (Variables|Default|GetMultiplier)) (Variables|Default|GetScore))))
  (return _output_get))

(fn GetSaveGameData
  (bind _current_save_object (Variables|Default|GetCurrent_Save_Object)
    (:then
      (return _current_save_object))
    (:else
      (bind _returnvalue (SaveGame|DoesSaveGameExist (Variables|Default|GetHigh_Score_Save_Name)))
      (if _returnvalue
        (bind _returnvalue_2 (SaveGame|LoadGamefromSlot (Variables|Default|GetHigh_Score_Save_Name)))
        (bind _ashigh_score_save_blueprint (Utilities|Casting|CastToHigh_Score_Save_Blueprint _returnvalue_2)
          (:then
            (Default|SortSaveData _ashigh_score_save_blueprint)
            (bind _output_get (Variables|Default|SetCurrent_Save_Object _ashigh_score_save_blueprint))
            (return _output_get))
          (:CastFailed
            _))
        (else
          (bind _returnvalue_3 (SaveGame|CreateSaveGameObject "/Game/Blueprints/High_Score_Save_Blueprint.High_Score_Save_Blueprint_C"))
          (bind _ashigh_score_save_blueprint_2 (Utilities|Casting|CastToHigh_Score_Save_Blueprint _returnvalue_3)
            (:then
              (bind _output_get_2 (Variables|Default|SetCurrent_Save_Object _ashigh_score_save_blueprint_2))
              (return _output_get_2))
            (:CastFailed
              _))))
      (return 0))))