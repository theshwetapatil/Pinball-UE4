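; High score save Blueprint that maintains a leaderboard of score structs in the SaveStruct array, capped at the top four.
; AddHighScore appends a new entry, calls SortSaveData, then trims the array.
; SortSaveData runs a descending selection sort, repeatedly moving the result of DetermineHighestScoreValue into a temporary array that replaces SaveStruct.
; DetermineLowestScoreValue similarly returns the lowest entry and index, but nothing here calls it.
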(fn DetermineLowestScoreValue
  (for (_array_element _array_index) (Variables|Default|GetSave_Struct) ; Check score of each struct
    (if (== _array_index 0)
      (LocalVariables|SetLowest_Score (.score _array_element)) ; Set loewest score \nto be equal to that of \nthe current index
      (LocalVariables|SetLowest_Index _array_index) ; Set loewest index \nto be equal to\nthe current index
      (elif (< (.score _array_element) (LocalVariables|GetLowest_Score))
        (LocalVariables|SetLowest_Score (.score _array_element)) ; Set loewest score \nto be equal to that of \nthe current index
        (LocalVariables|SetLowest_Index _array_index) ; Set loewest index \nto be equal to\nthe current index
      )))
  (return (Utilities|Array|Get(acopy) (Variables|Default|GetSave_Struct) (LocalVariables|GetLowest_Index)) (LocalVariables|GetLowest_Index)))

(fn DetermineHighestScoreValue
  (for (_array_element _array_index) (Variables|Default|GetSave_Struct) ; Check score of each struct
    (if (== _array_index 0)
      (LocalVariables|SetHighest_Score (.score _array_element)) ; Set loewest score \nto be equal to that of \nthe current index
      (LocalVariables|SetHighest_Index _array_index) ; Set loewest index \nto be equal to\nthe current index
      (elif (> (.score _array_element) (LocalVariables|GetHighest_Score))
        (LocalVariables|SetHighest_Score (.score _array_element)) ; Set loewest score \nto be equal to that of \nthe current index
        (LocalVariables|SetHighest_Index _array_index) ; Set loewest index \nto be equal to\nthe current index
      )))
  (return (Utilities|Array|Get(acopy) (Variables|Default|GetSave_Struct) (LocalVariables|GetHighest_Index)) (LocalVariables|GetHighest_Index)))

(fn SortSaveData
  (while (> (Utilities|Array|Length (Variables|Default|GetSave_Struct)) 0)
    (bind (_highest_score_struct _highest_score_index) (CallFunction|DetermineHighestScoreValue))
    (Utilities|Array|Add (LocalVariables|GetTemp_Save_Struct) _highest_score_struct)
    (Utilities|Array|RemoveIndex (Variables|Default|GetSave_Struct) _highest_score_index))
  (Variables|Default|SetSave_Struct (LocalVariables|GetTemp_Save_Struct)))

(fn AddHighScore
  (params (New_Score :type High%20Score%20Struct%20Structure))
  (bind _save_struct (Variables|Default|GetSave_Struct))
  (Utilities|Array|Add (Variables|Default|GetSave_Struct) New_Score)
  (CallFunction|SortSaveData)
  (Utilities|Array|Resize _save_struct (Math|Integer|Min(Integer) 4 (Utilities|Array|Length _save_struct))))