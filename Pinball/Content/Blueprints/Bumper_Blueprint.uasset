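; Pinball bumper actor that kicks an overlapping Ball_Blueprint away from itself and awards score through the pinball game mode.
; Overlap calls Bump, which applies a velocity-change impulse along the bumper-to-ball direction, plays an attached hit sound and spawns sparks.
; The Bump_Lerp timeline then drives the mechanism's vertical movement, point light intensity and emissive boost on a dynamic material created in the construction script.
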(event Custom|Bump
  (params (Ball :type Ball%20Blueprint%20Object%20Reference))
  (Physics|AddImpulse (Variables|/Game/Blueprints/Ball_Blueprint.Ball_Blueprint_C|GetBall Ball) (* (Math|Vector|GetUnitDirection(Vector) (Transformation|GetActorLocation) (Transformation|GetActorLocation Ball)) 2.5e+03) "None" true) ; On Add Impulse play Bump_Lerp from the start
  (Audio|SpawnSoundAttached "/Game/Assets/Sounds/Bumper_Hit.Bumper_Hit" (Variables|Default|GetBumperMesh)) ; Play the sound on Bumper Mesh/\nat the Bumper Mesh's location
  (bind _aspinball_game_mode_blueprint (Utilities|Casting|CastToPinball_Game_Mode_Blueprint (Game|GetGameMode))
    (:then
      (Default|AddScore _aspinball_game_mode_blueprint 1e+01))
    (:CastFailed
      _))
  (Effects|SpawnEmitteratLocation "/Game/Assets/Bumper_Sparks_ParticleSystem.Bumper_Sparks_ParticleSystem" (Transformation|GetWorldLocation (Variables|Default|GetBumperMechanism)))
  (bind _bump_alpha (Timeline|Bump_Lerp PlayFromStart) ; When Update runs, Bump Alpha changes
    (:Update
      (Transformation|SetRelativeLocation (Variables|Default|GetBumperMechanism) (Math|Vector|Lerp(Vector) "0, 0, 0" "0, 0,-70.000000" _bump_alpha) false false) ; To move Bumper Mechanism up and down
      (Rendering|Components|Light|SetIntensity (Variables|Default|GetPointLight) (Math|Float|Lerp 0.0 5e+03 _bump_alpha))
      (Rendering|Material|SetScalarParameterValue (Variables|Default|GetBumper_Top_MID) "Emissive_Boost" (Math|Float|Lerp 0.0 2e+01 _bump_alpha) :!class /Script/Engine.MaterialInstanceDynamic) ; Refers to the individual number(Emissive Boost)
    )))

(event EventBeginPlay)

(event Collision|EventActorBeginOverlap
  (params (OtherActor :type Actor%20Object%20Reference))
  (bind _asball_blueprint (Utilities|Casting|CastToBall_Blueprint OtherActor)) ; Check for collision
  (CallFunction|Bump _asball_blueprint) ; Check whether it's a Ball
)

(event EventTick
  (params (DeltaSeconds :type Float%20%28single-precision%29)))

(fn ConstructionScript
  (bind _returnvalue (Rendering|Material|CreateDynamicMaterialInstance (Variables|Default|GetBumperMesh) 1 0 :!class /Script/Engine.PrimitiveComponent)) ; Gets the element index specified ,\ncreates the dynamic material instance of it\nand then applies it to the mesh\n1: Top section of the mesh\n0: Base section of the mesh
  (Variables|Default|SetBumper_Top_MID _returnvalue) ; Store reference to the dynamic material
)