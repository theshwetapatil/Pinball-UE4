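; Plunger actor for launching a ball, with charge and release motion plus a ball spawn point.
; Charge_Plunger plays a timeline that lerps the plunger mesh along its local Y axis.
; Stop_Charge halts the timeline and quickly moves the mesh back to rest with MoveComponentTo, applying no force itself.
; GetBallSpawnLocation converts the relative BallLocation to world space through the actor transform.
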(event Custom|Charge_Plunger
  (bind _charge_alpha (Timeline|Charge_Timeline PlayFromStart)
    (:Update
      (Transformation|SetRelativeLocation (Variables|Default|GetPlunger_Mesh) (Math|Vector|Lerp(Vector) "0, 0, 0" "0,150.000000, 0" _charge_alpha) false false))))

(event Custom|Stop_Charge
  (Utilities|FlowControl|Sequence
    (:then_0
      (bind _charge_alpha (Timeline|Charge_Timeline Stop)
        (:Update
          (Transformation|SetRelativeLocation (Variables|Default|GetPlunger_Mesh) (Math|Vector|Lerp(Vector) "0, 0, 0" "0,150.000000, 0" _charge_alpha) false false))))
    (:then_1
      (Components|MoveComponentTo (Variables|Default|GetPlunger_Mesh) "0, 0, 0" "0, 0, 0" false false 0.1 false))))

(event EventBeginPlay)

(event Collision|EventActorBeginOverlap
  (params (OtherActor :type Actor%20Object%20Reference)))

(event EventTick
  (params (DeltaSeconds :type Float%20%28single-precision%29)))

(fn ConstructionScript)

(fn GetBallSpawnLocation
  (return (Math|Transform|TransformLocation (Transformation|GetActorTransform) (Variables|Default|GetBall_Location))) ; Return Position in the world
)