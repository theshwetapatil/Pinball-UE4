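; Pinball drop target set that spells an uppercased word with lettered targets and rewards clearing them.
; The construction script spawns one Drop_Target_Blueprint child actor per character, spacing them between Post1 and Post2, and binds each target's OnDrop event.
; Process_Drop_Targets decrements a counter and raises the game mode's Multiplier when it reaches zero.
; The game mode's OnGameReset restores the counter to the word length.
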(event Custom|Process_Drop_Targets
  (bind _result (Math|Integer|DecrementInt (Variables|Default|GetTarget_Counter))
    (:%20%20
      (if (== _result 0)
        (bind _aspinball_game_mode_blueprint (Utilities|Casting|CastToPinball_Game_Mode_Blueprint (Game|GetGameMode)))
        (Math|Float|IncrementFloat (Variables|/Game/Blueprints/Pinball_Game_Mode_Blueprint.Pinball_Game_Mode_Blueprint_C|GetMultiplier _aspinball_game_mode_blueprint))))))

(event Custom|Reset_Drop_Target_Counter
  (Variables|Default|SetTarget_Counter (Utilities|String|Len (Variables|Default|GetDrop_Target_String))))

(event EventBeginPlay
  (|CallParentFunction)
  (bind _aspinball_game_mode_blueprint (Utilities|Casting|CastToPinball_Game_Mode_Blueprint (Game|GetGameMode)))
  (EventDispatchers|BindEventtoOnGameReset _aspinball_game_mode_blueprint (delegate Custom|Reset_Drop_Target_Counter)))

(event Collision|EventActorBeginOverlap
  (params (OtherActor :type Actor%20Object%20Reference))
  (|CallParentFunction OtherActor) ; This node is disabled and will not be called.\nDrag off pins to build functionality.
)

(event EventTick
  (params (DeltaSeconds :type Float%20%28single-precision%29))
  (|CallParentFunction DeltaSeconds) ; This node is disabled and will not be called.\nDrag off pins to build functionality.
)

(fn ConstructionScript
  (bind _post1 (Variables|Default|GetPost1))
  (bind _returnvalue (Math|Vector|GetForwardVector _post1))
  (|CallParentFunction)
  (bind _output_get (Variables|Default|SetDrop_Target_String (Class|KismetStringLibrary|ToUpper (Variables|Default|GetDrop_Target_String))))
  (for (_array_element _array_index) (Utilities|String|GetCharacterArrayfromString _output_get) ; Creates child actor component,\nevery time it iterates through
    (bind _returnvalue_2 (AddComponent|AddChildActorComponent false (Math|Transform|MakeTransform (+ (* _returnvalue (* (+ _array_index 1) (/ (Math|Vector|VectorLength (- (Variables|/Script/Engine.SceneComponent|GetRelativeLocation (Variables|Default|GetPost1)) (Variables|/Script/Engine.SceneComponent|GetRelativeLocation (Variables|Default|GetPost2)))) (Math|Conversions|ToFloat(Integer) (+ (Utilities|Array|Length (Utilities|String|GetCharacterArrayfromString _output_get)) 1))))) (* _returnvalue 2e+01)) (Variables|/Script/Engine.SceneComponent|GetRelativeRotation _post1) "1,1,1"))) ; Spawns a new actor that's parented to DT_Mesh,\nas if it was a component of this actor
    (bind _asdrop_target_blueprint (Utilities|Casting|CastToDrop_Target_Blueprint (Variables|/Script/Engine.ChildActorComponent|GetChildActor _returnvalue_2)))
    (bind _output_get_2 (Variables|/Game/Blueprints/Drop_Target_Blueprint.Drop_Target_Blueprint_C|SetDrop_Letter _asdrop_target_blueprint _array_element))
    (Rendering|Components|TextRender|SetText (Variables|/Game/Blueprints/Drop_Target_Blueprint.Drop_Target_Blueprint_C|GetTextRender _asdrop_target_blueprint) (Utilities|Text|ToText(String) _output_get_2))
    (EventDispatchers|BindEventtoOnDrop _asdrop_target_blueprint (EventDispatchers|CreateEvent :!event Custom|Process_Drop_Targets))))